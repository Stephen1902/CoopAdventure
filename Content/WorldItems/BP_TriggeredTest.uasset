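; BP_TriggeredTest is a triggered world item that cycles through a list of colours and reports whether it shows the winning colour.
; Each activation advances the wrapping colour index, and StateHasChanged fires only when the match against ColourToWin flips CurrentState.
; A RepNotify on ReplicatedColour pushes each new colour to a dynamic material instance created and initialised at BeginPlay.
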(event `self.ReceiveBeginPlay`
  (bind _meshcomponent (`self.MeshComponent`))
  (bind _returnvalue (`PrimitiveComponent.CreateDynamicMaterialInstance` _meshcomponent 0 null "None"))
  (set `self.MatInstanceRef` _returnvalue)
  (`PrimitiveComponent.SetMaterial` _meshcomponent 0 _returnvalue)
  (`MaterialInstanceDynamic.SetVectorParameterValue` (`self.MatInstanceRef`) "DiffuseColor" (`|GetArrayItem` (`self.ColoursToDisplay`) (`self.ColourIndex`))))

(event `self.BPDealWithActivatedChanged`
  (params (BoolOut :type Boolean))
  (bind _output (`|GetArrayItem` (`self.ColoursToDisplay`) (`self.ColourIndex`)))
  (if BoolOut
    (bind _result (`/Engine/EditorBlueprintResources/StandardMacros.IncrementInt` (`self.ColourIndex`))
      (:`  `
        (set `self.ColourIndex` (mod _result (`KismetArrayLibrary.Array_Length` (`self.ColoursToDisplay`))))
        (set `self.ReplicatedColour` _output)
        (if (== _output (`self.ColourToWin`))
          (if (not (`self.CurrentState`))
            (set `self.CurrentState` true)
            (`self.StateHasChanged` (`self.CurrentState`) :!label _label))
          (elif (`self.CurrentState`)
            (set `self.CurrentState` false)
            (goto _label)))))))

(fn `OnRep_ReplicatedColour`
  (`MaterialInstanceDynamic.SetVectorParameterValue` (`self.MatInstanceRef`) "DiffuseColor" (`self.ReplicatedColour`)))

(fn `UserConstructionScript`)