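; BP_6SideNumbers is a world item that acts as a six-value number selector, with one number serving as its trigger.
; Each activation-changed event advances CurrentNumber, wrapping from 6 back to 1, then compares it with TriggerNumber.
; When the match result differs from CurrentState, it stores the new state and passes it to StateHasChanged.
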(event `self.BPDealWithActivatedChanged`
  (params (BoolOut :type Boolean))
  (if (== (`self.CurrentNumber`) 6)
    (set `self.CurrentNumber` 1)
    (else
      (bind _result (`/Engine/EditorBlueprintResources/StandardMacros.IncrementInt` (`self.CurrentNumber`))
        (:`  `
          (set `self.CurrentNumber` _result)))))
  (bind _matches (`self.Check if Matches`))
  (if (!= _matches (`self.CurrentState`))
    (bind _output_get (set `self.CurrentState` _matches))
    (`self.StateHasChanged` _output_get)))

(fn `Check if Matches`
  (returns (Matches :type Boolean))
  (return (== (`self.CurrentNumber`) (`self.TriggerNumber`))))

(fn `UserConstructionScript`)