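; Test interactable world actor that swings like a door through 110 degrees of yaw.
; BeginPlay gives its Rotation component the two travel points, and Interactwith prints the interacting character's name and enables that component's movement.
; A separate CloseDoor event reverses a yaw Timeline and re-arms itself by timer, but nothing else here calls it.
; Server and multicast interaction events are stubs, with their authority-check wiring disconnected.
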(event `self.ReceiveBeginPlay`
  (`RotationComponent.SetTravelPoints` :`self` (`self.Rotation`) :`RotPoint2` (struct :`Yaw` 110.0)))

(event `InteractionInterface.InteractWith`
  (params (CharacterWhoInteracted :type "TP_FirstPersonCharacter Object Reference"))
  (`KismetSystemLibrary.PrintString` (`KismetSystemLibrary.GetDisplayName` CharacterWhoInteracted))
  (`RotationComponent.SetCanMove` (`self.Rotation`) true))

(event `InteractMulticast`)

(event `InteractOnServer`
  (`self.InteractMulticast`))

(event `CloseDoor`
  (bind (_direction _newtrack_0) (`Timeline|Timeline` :!via `Reverse`)
    (:`Update`
      (`SceneComponent.K2_SetRelativeRotation` (`self.MeshComp`) (`KismetMathLibrary.MakeRotator` 0.0 0.0 (* _newtrack_0 110.0)) false false))
    (:`Finished`
      (`KismetSystemLibrary.K2_SetTimerDelegate` (delegate `CloseDoor`) 5.0))))

(fn `UserConstructionScript`)